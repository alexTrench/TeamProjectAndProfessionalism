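; CoverSpot is an actor that marks a cover position and exposes checks for judging it relative to the player.
; Every Tick it sets Available to false while CharacterInCover is valid, and true otherwise.
; ArrowIsFacingPlayer uses a dot product to test whether the Arrow's forward vector opposes the player character's forward vector, ignoring relative position.
; InSuitableRangeFromPlayer tests whether the player's distance lies within a given minimum and maximum.
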(event `self.ReceiveTick`
  (params (DeltaSeconds :type "Float (single-precision)"))
  ;[1 1 1] Set cover spot availability
  (if (`KismetSystemLibrary.IsValid` (`self.CharacterInCover`))
    (set `self.Available` false)
    (else
      (set `self.Available` true))))

(fn `ArrowIsFacingPlayer`
  (returns (ReturnValue :type Boolean))
  (return (not (>= (`KismetMathLibrary.Dot_VectorVector` (`SceneComponent.GetForwardVector` (`self.Arrow`)) (`self.GetActorForwardVector` (`GameplayStatics.GetPlayerCharacter` 0))) 0.0))))

(fn `InSuitableRangeFromPlayer`
  (params (MinRange :type "Float (double-precision)") (MaxRange :type "Float (double-precision)"))
  (returns (ReturnValue :type Boolean))
  (bind _returnvalue (`KismetMathLibrary.VSize` (- (`self.K2_GetActorLocation`) (`self.K2_GetActorLocation` (`GameplayStatics.GetPlayerCharacter` 0)))))
  (return (and (>= _returnvalue MinRange) (<= _returnvalue MaxRange))))

(fn `UserConstructionScript`)