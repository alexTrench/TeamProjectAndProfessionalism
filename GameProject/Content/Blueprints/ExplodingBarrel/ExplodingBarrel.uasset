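; Explosive barrel that takes randomized bullet damage, catches fire when badly damaged and explodes at zero health or when its fuse timer expires.
; While burning, Tick drains health from nearby characters and runs the timer.
; Explode plays effects, applies radial falloff damage and chain-reacts, detonating inner-radius barrels instantly and igniting outer ones.
; It also makes noise and sets nearby shooter AI to combat against the player before destroying itself.
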(event `/Game/Interfaces/DamageInterface.TakeDamage`
  (params (DamageMin :type "Float (single-precision)") (DamageMax :type "Float (single-precision)") (CriticalShotChance :type "Float (single-precision)") (HitBoneName :type Name) (DamageInstigator :type "Actor Object Reference"))
  ;[1 1 1] Take bullet damage
  (`self.CalculateBarrelHealth` DamageMin DamageMax))

(event `self.ReceiveTick`
  (params (DeltaSeconds :type "Float (single-precision)"))
  (if (not (`self.Exploding`))
    (`|ExecutionSequence`
      (:`then_0`
        ;[1 1 1] Start explosion timer after barrel has taken damage
        (if (`self.StartTimer`)
          (`|ExecutionSequence`
            (:`then_0`
              ;;[1 1 1] Start timer if not already started
              (if (not (`self.TimerStarted`))
                (set `self.TimerStart` (`KismetSystemLibrary.GetGameTimeInSeconds`))
                (set `self.TimerStarted` true)))
            (:`then_1`
              ;;[1 1 1] Increment timer
              (set `self.CurrentTimer` (- (`KismetSystemLibrary.GetGameTimeInSeconds`) (`self.TimerStart`))))
            (:`then_2`
              ;;[1 1 1] Explode barrel if timer is reached
              (if (>= (`self.CurrentTimer`) (`self.TimerLimit`))
                (`self.Explode`))))))
      (:`then_1`
        ;[1 1 1] If barrel is on fire, damage players in radius
        (if (`self.Damaged`)
          (`|ExecutionSequence`
            (:`then_0`
              (`/Engine/EditorBlueprintResources/StandardMacros.DoOnce` false
                (:`Completed`
                  (`ActorComponent.Activate` (`self.Fire`) false))))
            (:`then_1`
              (bind _outactors (`KismetSystemLibrary.SphereOverlapActors` (`SceneComponent.K2_GetComponentLocation` (`self.Fire`)) (`self.FireRadius`) (`|MakeArray` "ObjectTypeQuery3" :!type "EObjectTypeQuery Enum") "/Game/Player/CharacterBase.CharacterBase_C"))
              (for _array_element _outactors
                (bind _ascharacter_base (cast `/Game/Player/CharacterBase` _array_element))
                (set `/Game/Player/CharacterBase.Health` (- (`/Game/Player/CharacterBase.Health` _ascharacter_base) 0.001) _ascharacter_base)))))))))

(fn `BarrelWithinInnerRadius`
  (params (ExplodingBarrel :type "/Game/Blueprints/ExplodingBarrel/ExplodingBarrel Object Reference"))
  (returns (ReturnValue :type Boolean))
  (return (<= (`KismetMathLibrary.VSize` (- (`self.K2_GetActorLocation` ExplodingBarrel) (`self.K2_GetActorLocation`))) (/ (`self.ExplosionDamageRadius`) 2.0))))

(fn `CalculateBarrelHealth`
  (params (DamageMin :type "Float (double-precision)") (DamageMax :type "Float (double-precision)"))
  (locals (Damage :type "Float (double-precision)"))
  (set `local.Damage` (`KismetMathLibrary.RandomFloatInRange` DamageMin DamageMax))
  (bind _output_get (set `self.Health` (- (`self.Health`) (`local.Damage`))))
  (if (and (< _output_get 1.0) (not (`self.Damaged`)))
    (set `self.Damaged` true)
    (set `self.StartTimer` true))
  ;[1 1 1] Check if barrel health <=0.0. If so then explode
  (if (<= (`self.Health`) 0.0)
    (set `self.Health` 0.0)
    (`self.Explode`)))

(fn `Explode`
  (bind _returnvalue (`self.K2_GetActorLocation`))
  (bind _explosiondamageradius (`self.ExplosionDamageRadius`))
  (set `self.Exploding` true)
  (bind _returnvalue_2 (`GameplayStatics.SpawnEmitterAtLocation` "/Game/Blueprints/ExplodingBarrel/P_Explosion.P_Explosion" (`self.K2_GetActorLocation`)))
  (`SceneComponent.SetRelativeScale3D` _returnvalue_2 (6.5 6.5 6.5))
  (`GameplayStatics.PlaySoundAtLocation` "/Game/Sounds/Explosion01.Explosion01" _returnvalue)
  (`self.MakeNoise` 1.0 (`GameplayStatics.GetPlayerCharacter` 0) _returnvalue 2000.0)
  (`GameplayStatics.ApplyRadialDamageWithFalloff` (`self.ExplosionDamage`) 0.1 (`self.K2_GetActorLocation`) (/ _explosiondamageradius 2.0) _explosiondamageradius 1.0 "/Script/Engine.DamageType" (`|MakeArray` self :!type "Actor Object Reference") self (`self.GetInstigatorController`))
  (`|ExecutionSequence`
    (:`then_0`
      ;[1 1 1] Explode all barrels in inner radius and damage barrels in inner radius
      (bind _outactors (`KismetSystemLibrary.SphereOverlapActors` (`self.K2_GetActorLocation`) (`self.ExplosionDamageRadius`) (`|MakeArray` "ObjectTypeQuery1" :!type "EObjectTypeQuery Enum") "ExplodingBarrel_C" (`|MakeArray` self :!type "Actor Object Reference")))
      (for _array_element _outactors
        (bind _asexploding_barrel (cast `/Game/Blueprints/ExplodingBarrel/ExplodingBarrel` _array_element))
        (if (not (`/Game/Blueprints/ExplodingBarrel/ExplodingBarrel.Exploding` _asexploding_barrel))
          (if (`self.BarrelWithinInnerRadius` _asexploding_barrel)
            (`self.Explode` _asexploding_barrel)
            (else
              (set `/Game/Blueprints/ExplodingBarrel/ExplodingBarrel.Damaged` true _asexploding_barrel)
              (set `/Game/Blueprints/ExplodingBarrel/ExplodingBarrel.StartTimer` true _asexploding_barrel))))))
    (:`then_1`
      ;[1 1 1] Alert AI within radius
      (bind _outactors_2 (`KismetSystemLibrary.SphereOverlapActors` (`self.K2_GetActorLocation` self) 4000.0 (`|MakeArray` "ObjectTypeQuery3" :!type "EObjectTypeQuery Enum") "/Game/AI/Shooter/AI_ShooterCharacter.AI_ShooterCharacter_C" (`|MakeArray` self :!type "Actor Object Reference")))
      (for _array_element_2 _outactors_2
        (bind _asai_shooter_character (cast `/Game/AI/Shooter/AI_ShooterCharacter` _array_element_2))
        (`/Game/AI/Shooter/AI_ShooterCharacter.SetToCombatStatus` _asai_shooter_character (`GameplayStatics.GetPlayerCharacter` 0)))
      (`self.K2_DestroyActor`))))

(fn `UserConstructionScript`
  (`SphereComponent.SetSphereRadius` (`self.ExplosionRadius`) (`self.ExplosionDamageRadius`) true))