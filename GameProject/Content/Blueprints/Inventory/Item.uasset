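; Base pickup item that spins until collected and is picked up with E.
; Sphere overlap by anything but AI shooters enables input and shows a HUD prompt.
; Pickup plays a sound, makes noise, then branches on class: health packs raise a count, duplicate weapons and ammo refill reserve ammo.
; New weapons and the first health pack join the player's Inventory, hidden and attached to the spine socket.
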(event `self.ReceiveTick`
  (params (DeltaSeconds :type "Float (single-precision)"))
  (if (not (`self.PickedUp`))
    ;[0.114 0.1048 0.8385] Making the item spin when not picked up
    (`self.K2_SetActorTransform` self (`KismetMathLibrary.MakeTransform` (.location (`self.GetTransform` self)) (`KismetMathLibrary.MakeRotator` (.roll (.rotation (`self.GetTransform` self))) (.pitch (.rotation (`self.GetTransform` self))) (+ (.yaw (.rotation (`self.GetTransform` self))) 1.0)) (.scale (`self.GetTransform` self))) false false)
    (else
      ;[1 1 1] Destroy point light when PickedUp
      (`/Engine/EditorBlueprintResources/StandardMacros.DoOnce` false
        (:`Completed`
          (`SceneComponent.K2_DetachFromComponent` (`self.PointLight`) "KeepRelative" "KeepRelative" "KeepRelative" true)
          (`ActorComponent.K2_DestroyComponent` (`self.PointLight`)))))))

(event `self.Sphere.OnComponentBeginOverlap`
  (params (OverlappedComponent :type "PrimitiveComponent Object Reference") (OtherActor :type "Actor Object Reference") (OtherComp :type "PrimitiveComponent Object Reference") (OtherBodyIndex :type Integer) (bFromSweep :type Boolean) (SweepResult :type "HitResult Structure (by ref)"))
  ;[1 1 1] Sphere overlap
  (if (and (!= (`GameplayStatics.GetObjectClass` OtherActor) "/Game/AI/Shooter/AI_ShooterCharacter.AI_ShooterCharacter_C") (not (`self.PickedUp`)))
    (`self.EnableInput` (`GameplayStatics.GetPlayerController` 0))
    (bind _asplayer_character (cast `/Game/Player/PlayerCharacter` (`GameplayStatics.GetPlayerCharacter` 0)))
    (bind _pickuptexthud (`/Game/Blueprints/HUD/HUD.PickupTextHUD` (`/Game/Player/PlayerCharacter.HUDReference` _asplayer_character)))
    (`TextBlock.SetText` _pickuptexthud (`KismetTextLibrary.Conv_StringToText` (`KismetStringLibrary.Concat_StrStr` "Press [E] to pickup " (`KismetTextLibrary.Conv_TextToString` (`self.ItemName`)))))
    (`Widget.SetVisibility` _pickuptexthud "Visible")))

(event `self.Sphere.OnComponentEndOverlap`
  (params (OverlappedComponent :type "PrimitiveComponent Object Reference") (OtherActor :type "Actor Object Reference") (OtherComp :type "PrimitiveComponent Object Reference") (OtherBodyIndex :type Integer))
  ;[1 1 1] Sphere overlap
  (if (!= (`GameplayStatics.GetObjectClass` OtherActor) "/Game/AI/Shooter/AI_ShooterCharacter.AI_ShooterCharacter_C")
    (`self.DisableInput` (`GameplayStatics.GetPlayerController` 0))
    (bind _asplayer_character (cast `/Game/Player/PlayerCharacter` (`GameplayStatics.GetPlayerCharacter` 0)))
    (`Widget.SetVisibility` (`/Game/Blueprints/HUD/HUD.PickupTextHUD` (`/Game/Player/PlayerCharacter.HUDReference` _asplayer_character)) "Hidden")))

(event `Key|E`
  (params (Key :type "Key Structure"))
  (bind _returnvalue (`self.K2_GetActorLocation`))
  (bind _returnvalue_2 (`GameplayStatics.GetObjectClass` self))
  ;[1 1 1] Item pickup
  ;;[1 1 1] Check if item is already in player's inventory
  (:`Pressed`
    (if (not (`self.PickedUp`))
      (set `self.PickedUp` true)
      (set `self.AlreadyInInventory` false)
      (`PrimitiveComponent.SetCollisionEnabled` (`self.Sphere`) "NoCollision")
      (`GameplayStatics.PlaySoundAtLocation` "/Game/Sounds/Guns/Other/WeaponPickup.WeaponPickup" _returnvalue)
      (`self.MakeNoise` 0.5 (`GameplayStatics.GetPlayerCharacter` 0) _returnvalue 5.0)
      (bind _asplayer_character (cast `/Game/Player/PlayerCharacter` (`GameplayStatics.GetPlayerCharacter` 0)))
      (bind _inventory (`/Game/Player/PlayerCharacter.Inventory` _asplayer_character))
      (for _array_element _inventory
        (if (== (`GameplayStatics.GetObjectClass` _array_element) (`GameplayStatics.GetObjectClass` self))
          (set `self.AlreadyInInventory` true)))
      (if (`self.AlreadyInInventory`)
        ;;[1 1 1] If so and it's a health pack, add 1 to HealthPackCount
        (if (== _returnvalue_2 "/Game/Blueprints/HealthPack/HealthPack.HealthPack_C")
          (`/Engine/EditorBlueprintResources/StandardMacros.IncrementInt` (`/Game/Player/PlayerCharacter.HealthPackCount` _asplayer_character)
            (:`  `
              (`self.K2_DestroyActor`)))
          (else
            ;;[1 1 1] If so and it's a weapon, set max extra ammo for the weapon already in the inventory
            (for _array_element_2 _inventory
              (if (== _returnvalue_2 (`GameplayStatics.GetObjectClass` _array_element_2))
                (bind _asbase_weapon (cast `/Game/Blueprints/Weapons/BaseWeapon` _array_element_2))
                (set `/Game/Blueprints/Weapons/BaseWeapon.ExtraAmmo` (- (`/Game/Blueprints/Weapons/BaseWeapon.MaxAmmo` _asbase_weapon) (`/Game/Blueprints/Weapons/BaseWeapon.MaxMagazine` _asbase_weapon)) _asbase_weapon)
                (`self.K2_DestroyActor`)))))
        (elif (== (`GameplayStatics.GetObjectClass` self) "/Game/Blueprints/Ammo/Ammo.Ammo_C")
          ;;[1 1 1] If not and is ammo, add ammo to all weapons in inventory
          (for _array_element_3 _inventory
            (if (!= (`GameplayStatics.GetObjectClass` _array_element_3) "/Game/Blueprints/HealthPack/HealthPack.HealthPack_C")
              (bind _asbase_weapon_2 (cast `/Game/Blueprints/Weapons/BaseWeapon` _array_element_3))
              (set `/Game/Blueprints/Weapons/BaseWeapon.ExtraAmmo` (- (`/Game/Blueprints/Weapons/BaseWeapon.MaxAmmo` _asbase_weapon_2) (`/Game/Blueprints/Weapons/BaseWeapon.MaxMagazine` _asbase_weapon_2)) _asbase_weapon_2)
              (`self.K2_DestroyActor`)))
          (else
            ;;[1 1 1] If not and not ammo, add item to inventory
            (`KismetArrayLibrary.Array_Add` (`/Game/Player/PlayerCharacter.Inventory` _asplayer_character) self)
            (set `self.PickedUp` true)
            (if (!= (`GameplayStatics.GetObjectClass` self) "/Game/Blueprints/HealthPack/HealthPack.HealthPack_C")
              (bind _asbase_weapon_3 (cast `/Game/Blueprints/Weapons/BaseWeapon` self))
              (set `/Game/Blueprints/Weapons/BaseWeapon.WeaponOwner` _asplayer_character _asbase_weapon_3)
              (else
                (`/Engine/EditorBlueprintResources/StandardMacros.IncrementInt` (`/Game/Player/PlayerCharacter.HealthPackCount` _asplayer_character)
                  (:`  `
                    _))))
            (`SceneComponent.SetVisibility` (`self.DefaultSceneRoot`) false true)
            (`SceneComponent.K2_AttachToComponent` (`self.DefaultSceneRoot`) (`Character.Mesh` _asplayer_character) "spine_Socket" "KeepRelative" "KeepRelative" "KeepRelative" true)))))))

(fn `UserConstructionScript`)