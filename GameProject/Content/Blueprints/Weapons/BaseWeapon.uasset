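; Base weapon Blueprint for player and AI shooters, holding ammo and combat stats, a delayed noise-making reload, and empty fire events.
; Fire functions spawn a casing and a projectile carrying damage and crit data, with cone spread for hip or ADS.
; Player shots trace from the active shoulder camera, spawning there for hits within 850 units, otherwise at the muzzle.
; AI shots aim from the muzzle at the target's spine.
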(event `ForcedReloadBase`
  (params (SoundEffect :type "SoundBase Object Reference") (Delay :type "Float (double-precision)"))
  (bind _returnvalue (- (`self.MaxMagazine`) (`self.CurrentMagAmmo`)))
  (bind _returnvalue_2 (`SceneComponent.K2_GetComponentLocation` (`self.WeaponMesh`)))
  ;[1 1 1] Forced reload
  (if (and (< (`self.CurrentMagAmmo`) (`self.MaxMagazine`)) (> (`self.ExtraAmmo`) 0))
    (set `self.reloading` true)
    (`GameplayStatics.PlaySoundAtLocation` SoundEffect _returnvalue_2)
    (`self.MakeNoise` 0.5 (`GameplayStatics.GetPlayerCharacter` 0) _returnvalue_2 10.0)
    (`KismetSystemLibrary.Delay` Delay)
    (set `self.reloading` false)
    (if (> (`self.ExtraAmmo`) _returnvalue)
      (set `self.AmmoDifference` _returnvalue)
      (set `self.CurrentMagAmmo` (+ (`self.CurrentMagAmmo`) (`self.AmmoDifference`)))
      (set `self.ExtraAmmo` (- (`self.ExtraAmmo`) (`self.AmmoDifference`)))
      (else
        (set `self.AmmoDifference` _returnvalue)
        (set `self.CurrentMagAmmo` (+ (`self.CurrentMagAmmo`) (`self.ExtraAmmo`)))
        (set `self.ExtraAmmo` 0)))))

(event `ForcedReload`
  ;[1 1 1] Forced reload
)

(event `FireWeapon`
  ;[1 1 1] FireWeapon/StopFireWeapon
)

(event `StopFireWeapon`
  ;[1 1 1] FireWeapon/StopFireWeapon
)

(fn `DebugDisplayAmmo`
  (`KismetSystemLibrary.PrintString` (`KismetStringLibrary.Concat_StrStr` (`KismetStringLibrary.Conv_IntToString` (`self.CurrentMagAmmo`)) "/" (`KismetStringLibrary.Conv_IntToString` (`self.ExtraAmmo`))))
  (return))

(fn `DebugDisplayWeaponSpread`
  (locals (Spread :type "Float (double-precision)") (Rotation :type "Rotator Structure"))
  (bind _spread (`local.Spread`))
  (set `local.Rotation` (`self.K2_GetActorRotation`))
  (bind _asplayer_character (cast `/Game/Blueprints/Player/PlayerCharacter` (`self.WeaponOwner`))
    (:`then`
      (if (`/Game/Blueprints/Player/PlayerCharacter.AimingDownSights` _asplayer_character)
        (set `local.Spread` (`self.AimDownSightsSpread`))
        (else
          (set `local.Spread` (`self.HipFireSpread`))))
      (bind _leftcamera (`/Game/Blueprints/Player/PlayerCharacter.LeftCamera` _asplayer_character))
      (`KismetSystemLibrary.DrawDebugBox` (+ (`SceneComponent.K2_GetComponentLocation` _leftcamera) (* (`SceneComponent.GetForwardVector` _leftcamera) (`self.Range`))) (`KismetMathLibrary.MakeVector` 0.0 _spread _spread) (struct :`R` 1.0 :`G` 1.0 :`B` 1.0 :`A` 1.0) (`local.Rotation`) 1.0)
      (return))
    (:`CastFailed`
      (return))))

(fn `FireFromAI`
  (bind _returnvalue (`self.GetAIProjectileSpawn`))
  (bind _returnvalue_2 (`|SpawnActorFromClass` (`self.ProjectileClass`) _returnvalue "AlwaysSpawn" "OverrideRootScale" null (`self.WeaponOwner`)))
  (`/Game/Blueprints/Weapons/Projectiles/BaseProjectile.SetDamageInfo` _returnvalue_2 (`self.DamageMin`) (`self.DamageMax`) (`self.CriticalShotChance`))
  (`|SpawnActorFromClass` (`self.CasingClass`) (`SceneComponent.GetSocketTransform` (`self.WeaponMesh`) "Casing" "RTS_World") "AlwaysSpawn" "OverrideRootScale" null null)
  (return))

(fn `FireFromPlayer`
  (params (Range :type "Float (double-precision)"))
  (bind _returnvalue (`self.GetPlayerProjectileSpawn` Range))
  (bind _returnvalue_2 (`|SpawnActorFromClass` (`self.ProjectileClass`) _returnvalue "AlwaysSpawn" "OverrideRootScale" null (`self.WeaponOwner`)))
  (`/Game/Blueprints/Weapons/Projectiles/BaseProjectile.SetDamageInfo` _returnvalue_2 (`self.DamageMin`) (`self.DamageMax`) (`self.CriticalShotChance`))
  (`|SpawnActorFromClass` (`self.CasingClass`) (`SceneComponent.GetSocketTransform` (`self.WeaponMesh`) "Casing" "RTS_World") "AlwaysSpawn" "OverrideRootScale" null null)
  (return))

(fn `GetAIProjectileSpawn`
  (returns (ReturnValue :type "Transform Structure"))
  (locals (Spread :type "Float (double-precision)"))
  (bind _returnvalue (`SceneComponent.GetSocketLocation` (`self.WeaponMesh`) "Muzzle"))
  ;[1 1 1] Set local handles
  (bind _asai_shooter_character (cast `/Game/AI/Shooter/AI_ShooterCharacter` (`self.WeaponOwner`)))
  (if (`/Game/AI/Shooter/AI_ShooterCharacter.AimingDownSights` _asai_shooter_character)
    (bind _equippedweapon (`/Game/AI/Shooter/AI_ShooterCharacter.EquippedWeapon` _asai_shooter_character))
    (set `local.Spread` (`/Game/Blueprints/Weapons/BaseWeapon.AimDownSightsSpread` _equippedweapon))
    (else
      (set `local.Spread` (`/Game/Blueprints/Weapons/BaseWeapon.HipFireSpread` _equippedweapon))))
  (bind _returnvalue_2 (`SceneComponent.GetSocketLocation` (`Character.Mesh` (`/Game/AI/Shooter/AI_ShooterCharacter.TargetCharacter` _asai_shooter_character)) "spine_03"))
  (return (`KismetMathLibrary.MakeTransform` (.location (`KismetMathLibrary.MakeTransform` _returnvalue (`KismetMathLibrary.FindLookAtRotation` _returnvalue _returnvalue_2))) (`KismetMathLibrary.Conv_VectorToRotator` (`KismetMathLibrary.RandomUnitVectorInConeInDegrees` (- _returnvalue_2 _returnvalue) (`local.Spread`))))))

(fn `GetPlayerProjectileSpawn`
  (params (Range :type "Float (double-precision)"))
  (returns (ReturnValue :type "Transform Structure"))
  (locals (WeaponRange :type "Float (double-precision)") (PlayerCamera :type "CameraComponent Object Reference") (Spread :type "Float (double-precision)") (LocalDebug :type Boolean :default false))
  (bind _spread (`local.Spread`))
  (bind _spread_2 (`local.Spread`))
  (bind _playercamera (`local.PlayerCamera`))
  (bind _returnvalue (`SceneComponent.K2_GetComponentLocation` _playercamera))
  (bind _returnvalue_2 (`SceneComponent.GetSocketLocation` (`self.WeaponMesh`) "Muzzle"))
  (bind _returnvalue_3 (`SceneComponent.GetSocketLocation` (`self.WeaponMesh`) "Muzzle"))
  (bind _returnvalue_4 (`SceneComponent.K2_GetComponentLocation` (`local.PlayerCamera`)))
  ;[1 1 1] Set local handles
  (set `local.WeaponRange` Range)
  (bind _asplayer_character (cast `/Game/Blueprints/Player/PlayerCharacter` (`GameplayStatics.GetPlayerCharacter` 0)))
  (if (`/Game/Blueprints/Player/PlayerCharacter.CameraRightSide` _asplayer_character)
    (bind _aimingdownsights (`/Game/Blueprints/Player/PlayerCharacter.AimingDownSights` _asplayer_character))
    (if _aimingdownsights
      (set `local.PlayerCamera` (`/Game/Blueprints/Player/PlayerCharacter.RightZoomCamera` _asplayer_character))
      (else
        (set `local.PlayerCamera` (`/Game/Blueprints/Player/PlayerCharacter.RightCamera` _asplayer_character))))
    (elif _aimingdownsights
      (set `local.PlayerCamera` (`/Game/Blueprints/Player/PlayerCharacter.LeftZoomCamera` _asplayer_character))
      (else
        (set `local.PlayerCamera` (`/Game/Blueprints/Player/PlayerCharacter.LeftCamera` _asplayer_character)))))
  (bind _asbase_weapon (cast `/Game/Blueprints/Weapons/BaseWeapon` (`/Game/Blueprints/Player/PlayerCharacter.EquippedItem` _asplayer_character)))
  (if (`/Game/Blueprints/Player/PlayerCharacter.AimingDownSights` _asplayer_character)
    (set `local.Spread` (`/Game/Blueprints/Weapons/BaseWeapon.AimDownSightsSpread` _asbase_weapon))
    (else
      (set `local.Spread` (`/Game/Blueprints/Weapons/BaseWeapon.HipFireSpread` _asbase_weapon))))
  ;[1 1 1] Line trace from camera to centre of screen
  (bind (_outhit _returnvalue_5) (`KismetSystemLibrary.LineTraceSingle` _returnvalue (+ _returnvalue (* (`SceneComponent.GetForwardVector` _playercamera) (`local.WeaponRange`))) "TraceTypeQuery2"))
  (if _returnvalue_5
    (bind (_bblockinghit _binitialoverlap _time _distance _location _impactpoint _normal _impactnormal _physmat _hitactor _hitcomponent _hitbonename _hititem _faceindex _tracestart _traceend) (`GameplayStatics.BreakHitResult` _outhit))
    (if (<= (`KismetMathLibrary.VSize` (- (`SceneComponent.K2_GetComponentLocation` (`local.PlayerCamera`)) _impactpoint)) 850.0)
      (`|ExecutionSequence`
        (:`then_0`
          _)
        (:`then_1`
          ;[1 1 1] Line trace HIT
          (return (`KismetMathLibrary.MakeTransform` (.location (`KismetMathLibrary.MakeTransform` _returnvalue_4 (`KismetMathLibrary.FindLookAtRotation` _returnvalue_4 _impactpoint))) (`KismetMathLibrary.Conv_VectorToRotator` (`KismetMathLibrary.RandomUnitVectorInConeInDegrees` (- _impactpoint _returnvalue_4) (`local.Spread`)))))))
      (else
        (`|ExecutionSequence`
          (:`then_0`
            _)
          (:`then_1`
            (bind _returnvalue_6 (- _impactpoint _returnvalue_3))
            (return (`KismetMathLibrary.MakeTransform` (.location (`KismetMathLibrary.MakeTransform` _returnvalue_3 (`KismetMathLibrary.FindLookAtRotation` _returnvalue_3 _impactpoint))) (`KismetMathLibrary.Conv_VectorToRotator` (`KismetMathLibrary.RandomUnitVectorInConeInDegrees` _returnvalue_6 (`local.Spread`)))))))))
    ;;[1 1 1] Debug
    (if (`local.LocalDebug`)
      (`KismetSystemLibrary.DrawDebugSphere` _impactpoint 50.0 12 (struct :`G` 1.0 :`B` 0.909613 :`A` 1.0) 5.0)
      (`KismetSystemLibrary.DrawDebugConeInDegrees` _returnvalue_3 _returnvalue_6 250.0 _spread _spread 12 (struct :`R` 1.0 :`G` 1.0 :`B` 1.0 :`A` 1.0) 5.0))
    (else
      ;[1 1 1] Line trace NO HIT (Firing at sky OR out of range)
      (`|ExecutionSequence`
        (:`then_0`
          ;;[1 1 1] Debug
          (if (`local.LocalDebug`)
            (`KismetSystemLibrary.DrawDebugSphere` _traceend 50.0 12 (struct :`G` 0.962571 :`B` 1.0 :`A` 1.0) 5.0)
            (bind _returnvalue_7 (- _traceend _returnvalue_2))
            (`KismetSystemLibrary.DrawDebugConeInDegrees` _returnvalue_2 _returnvalue_7 250.0 _spread_2 _spread_2 12 (struct :`R` 1.0 :`G` 1.0 :`B` 1.0 :`A` 1.0) 5.0)))
        (:`then_1`
          (return (`KismetMathLibrary.MakeTransform` (.location (`KismetMathLibrary.MakeTransform` _returnvalue_2 (`KismetMathLibrary.FindLookAtRotation` _returnvalue_2 _traceend))) (`KismetMathLibrary.Conv_VectorToRotator` (`KismetMathLibrary.RandomUnitVectorInConeInDegrees` _returnvalue_7 (`local.Spread`))))))))))

(fn `SetWeaponAttributes`
  (params (CurrentMagAmmo :type Integer) (ExtraAmmo :type Integer) (MaxAmmo :type Integer) (MaxMagazine :type Integer) (DamageMin :type "Float (double-precision)") (DamageMax :type "Float (double-precision)") (CriticalShotChance :type "Float (double-precision)") (AimDownSightsSpread :type "Float (double-precision)") (HipFireSpread :type "Float (double-precision)") (Range :type "Float (double-precision)") (FireRate :type "Float (double-precision)"))
  (`|ExecutionSequence`
    (:`then_0`
      ;[1 1 1] Set ammo
      (set `self.CurrentMagAmmo` CurrentMagAmmo)
      (set `self.ExtraAmmo` ExtraAmmo)
      (set `self.MaxAmmo` MaxAmmo)
      (set `self.MaxMagazine` MaxMagazine))
    (:`then_1`
      ;[1 1 1] Set damage information (0.00 - 1.00)
      (set `self.DamageMin` DamageMin)
      (set `self.DamageMax` DamageMax)
      (set `self.CriticalShotChance` CriticalShotChance))
    (:`then_2`
      ;[1 1 1] Set spread (cm offset from centre of screen)
      (set `self.AimDownSightsSpread` AimDownSightsSpread)
      (set `self.HipFireSpread` HipFireSpread))
    (:`then_3`
      ;[1 1 1] Set range (cm) and fire rate (shot every X seconds)
      (set `self.Range` Range)
      (set `self.FireRate` FireRate))
    (:`then_4`
      (return))))

(fn `UserConstructionScript`)