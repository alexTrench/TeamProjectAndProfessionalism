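; Health pack item that restores the player's health when used and names itself for pickup text on BeginPlay.
; UseHealthPack adds its Health value to the PlayerCharacter's Health, caps the result at 1.0 and decrements that character's HealthPackCount.
; It then plays a sound at the pack's location and calls MakeNoise there with the player as instigator, emitting a short-range noise event.
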(event `UseHealthPack`
  (bind _returnvalue (`self.K2_GetActorLocation`))
  ;[1 1 1] UseHealthPack
  (bind _asplayer_character (cast `/Game/Player/PlayerCharacter` (`GameplayStatics.GetPlayerCharacter` 0)))
  (bind _returnvalue_2 (+ (`/Game/Player/CharacterBase.Health` _asplayer_character) (`self.Health`)))
  (if (> _returnvalue_2 1.0)
    (set `/Game/Player/CharacterBase.Health` 1.0 _asplayer_character)
    (else
      (set `/Game/Player/CharacterBase.Health` _returnvalue_2 _asplayer_character)))
  (`/Engine/EditorBlueprintResources/StandardMacros.DecrementInt` (`/Game/Player/PlayerCharacter.HealthPackCount` _asplayer_character)
    (:`  `
      (`GameplayStatics.PlaySoundAtLocation` "/Game/Sounds/PlayerSoundEffects/Other/Health_Pack.Health_Pack" _returnvalue)
      (`self.MakeNoise` 0.5 (`GameplayStatics.GetPlayerCharacter` 0) _returnvalue 5.0))))

(event `self.ReceiveBeginPlay`
  (`parent.ReceiveBeginPlay`)
  ;[1 1 1] Set PickupText
  (set `self.ItemName` "Health Pack"))

(fn `UserConstructionScript`)