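; Character base Blueprint that handles health, random-range weapon damage and death for player and enemy characters.
; Radial damage, commented as explosive barrels, and both health functions subtract from Health, clamp it at zero and set Dead.
; Enemy damage also switches on hit bone, recording headshots with fixed 1.0 damage.
; Non-lethal arm and torso hits cast self to AI_ShooterCharacter to set hit-reaction flags.
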(event `self.ReceiveRadialDamage`
  (params (DamageReceived :type "Float (single-precision)") (DamageType :type "DamageType Object Reference") (Origin :type "Vector Structure") (HitInfo :type "HitResult Structure (by ref)") (InstigatedBy :type "Controller Object Reference") (DamageCauser :type "Actor Object Reference"))
  ;[1 1 1] Explosive barrel damage
  (bind _output_get (set `self.Health` (- (`self.Health`) DamageReceived)))
  (if (<= _output_get 0.0)
    (set `self.Health` 0.0)
    (set `self.Dead` true)))

(fn `CalculateEnemyHealth`
  (params (DamageMin :type "Float (double-precision)") (DamageMax :type "Float (double-precision)") (CriticalShotChance :type "Float (double-precision)") (HitBoneName :type Name))
  (locals (Damage :type "Float (double-precision)"))
  (if (not (`self.Dead`))
    (set `local.Damage` (`KismetMathLibrary.RandomFloatInRange` DamageMin DamageMax))
    (`|ExecutionSequence`
      (:`then_0`
        (switch `name` HitBoneName
          (:`Default`
            (set `self.LastHitHeadshot` false))
          (:`Head`
            (set `self.LastHitHeadshot` true)))
        (switch `name` HitBoneName
          (:`Head`
            ;[1 1 1] Headshot
            (set `local.Damage` 1.0))
          (:`LeftArm`
            ;[1 1 1] LeftArm hit - Hit_React_1 animation
            (bind _asai_shooter_character (cast `/Game/AI/Shooter/AI_ShooterCharacter` self))
            (if (and (not (`/Game/AI/Shooter/AI_ShooterCharacter.Hit` _asai_shooter_character)) (> (- (`self.Health`) (`local.Damage`)) 0.0))
              (set `/Game/AI/Shooter/AI_ShooterCharacter.Hit` true _asai_shooter_character)
              (set `/Game/AI/Shooter/AI_ShooterCharacter.UpperarmLeftHit` true _asai_shooter_character)))
          (:`Spine2`
            ;[1 1 1] Spine2 hit - Hit_React_2 animation
            (bind _asai_shooter_character_2 (cast `/Game/AI/Shooter/AI_ShooterCharacter` self))
            (if (and (not (`/Game/AI/Shooter/AI_ShooterCharacter.Hit` _asai_shooter_character_2)) (> (- (`self.Health`) (`local.Damage`)) 0.0))
              (set `/Game/AI/Shooter/AI_ShooterCharacter.Hit` true _asai_shooter_character_2)
              (set `/Game/AI/Shooter/AI_ShooterCharacter.MidTorsoHit` true _asai_shooter_character_2)))
          (:`Spine1`
            ;[1 1 1] Spine1 hit - Hit_React_3 animation
            (bind _asai_shooter_character_3 (cast `/Game/AI/Shooter/AI_ShooterCharacter` self))
            (if (and (not (`/Game/AI/Shooter/AI_ShooterCharacter.Hit` _asai_shooter_character_3)) (> (- (`self.Health`) (`local.Damage`)) 0.0))
              (set `/Game/AI/Shooter/AI_ShooterCharacter.Hit` true _asai_shooter_character_3)
              (set `/Game/AI/Shooter/AI_ShooterCharacter.StomachHit` true _asai_shooter_character_3)))
          (:`RightArm`
            ;[1 1 1] RightArm hit - Hit_React_4 animation
            (bind _asai_shooter_character_4 (cast `/Game/AI/Shooter/AI_ShooterCharacter` self))
            (if (and (not (`/Game/AI/Shooter/AI_ShooterCharacter.Hit` _asai_shooter_character_4)) (> (- (`self.Health`) (`local.Damage`)) 0.0))
              (set `/Game/AI/Shooter/AI_ShooterCharacter.Hit` true _asai_shooter_character_4)
              (set `/Game/AI/Shooter/AI_ShooterCharacter.UpperarmRightHit` true _asai_shooter_character_4)))))
      (:`then_1`
        ;[1 1 1] Set health and check if character is dead
        (bind _output_get (set `self.Health` (- (`self.Health`) (`local.Damage`))))
        (if (<= _output_get 0.0)
          (set `self.Health` 0.0)
          (set `self.Dead` true))))))

(fn `CalculatePlayerHealth`
  (params (DamageMin :type "Float (double-precision)") (DamageMax :type "Float (double-precision)") (CriticalShotChance :type "Float (double-precision)") (HitBoneName :type Name))
  (locals (Damage :type "Float (double-precision)"))
  (if (not (`self.Dead`))
    (set `local.Damage` (`KismetMathLibrary.RandomFloatInRange` DamageMin DamageMax))
    ;[1 1 1] Set health and check if character is dead
    (bind _output_get (set `self.Health` (- (`self.Health`) (`local.Damage`))))
    (if (<= _output_get 0.0)
      (set `self.Health` 0.0)
      (set `self.Dead` true))))

(fn `UserConstructionScript`)