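; Interactable safe that the player opens and closes with E, yielding an Ammo pickup.
; A box overlap toggles the HUD prompt and input for the player.
; A FlipFlop plays or reverses a timeline that yaws an Arrow component as the door pivot, with a sound and MakeNoise call each way.
; A DoOnce on the timeline update spawns the Ammo at a hard-coded world location as the door first moves.
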(event `self.Box.OnComponentBeginOverlap`
  (params (OverlappedComponent :type "PrimitiveComponent Object Reference") (OtherActor :type "Actor Object Reference") (OtherComp :type "PrimitiveComponent Object Reference") (OtherBodyIndex :type Integer) (bFromSweep :type Boolean) (SweepResult :type "HitResult Structure (by ref)"))
  (bind _asplayer_character (cast `/Game/Blueprints/Player/PlayerCharacter` OtherActor))
  (bind _pickuptexthud (`/Game/Blueprints/HUD/HUD.PickupTextHUD` (`/Game/Blueprints/Player/PlayerCharacter.HUDReference` _asplayer_character)))
  (`TextBlock.SetText` _pickuptexthud "Press [E] to interact")
  (`Widget.SetVisibility` _pickuptexthud "Visible")
  (`self.EnableInput` (`GameplayStatics.GetPlayerController` 0)))

(event `self.Box.OnComponentEndOverlap`
  (params (OverlappedComponent :type "PrimitiveComponent Object Reference") (OtherActor :type "Actor Object Reference") (OtherComp :type "PrimitiveComponent Object Reference") (OtherBodyIndex :type Integer))
  (bind _asplayer_character (cast `/Game/Blueprints/Player/PlayerCharacter` OtherActor))
  (`Widget.SetVisibility` (`/Game/Blueprints/HUD/HUD.PickupTextHUD` (`/Game/Blueprints/Player/PlayerCharacter.HUDReference` _asplayer_character)) "Hidden")
  (`self.DisableInput` null))

(event `Key|E`
  (params (Key :type "Key Structure"))
  (bind _returnvalue (`GameplayStatics.GetPlayerCharacter` 0))
  (bind _returnvalue_2 (`GameplayStatics.GetPlayerCharacter` 0))
  (bind (_returnvalue_location _returnvalue_rotation) (`KismetMathLibrary.BreakTransform` (`self.GetTransform` (`self.Ammo`))))
  (:`Pressed`
    (`/Engine/EditorBlueprintResources/StandardMacros.FlipFlop`
      (:`A`
        (`GameplayStatics.PlaySound2D` "/Game/Sounds/WorldSounds/Safe/Safe_-_Open.Safe_-_Open")
        (`self.MakeNoise` _returnvalue_2 0.5 _returnvalue_2 (`self.K2_GetActorLocation` _returnvalue_2) 10.0 "None")
        (bind (_direction _dooropen) (`Timeline|Timeline_0` :!label _label)
          (:`Update`
            (`SceneComponent.K2_SetRelativeRotation` (`self.Arrow`) (`KismetMathLibrary.MakeRotator` 0.0 0.0 _dooropen) false false)
            (`/Engine/EditorBlueprintResources/StandardMacros.DoOnce` false
              (:`Completed`
                (`|SpawnActorFromClass` "/Game/Blueprints/Ammo/Ammo.Ammo_C" (`KismetMathLibrary.MakeTransform` (-7009.29248 8641.359375 -10015.435547) _returnvalue_rotation (0.477871 0.477871 0.477871)) "Undefined" "OverrideRootScale" null null))))))
      (:`B`
        (`GameplayStatics.PlaySound2D` "/Game/Sounds/WorldSounds/Safe/Safe_-_Close.Safe_-_Close")
        (`self.MakeNoise` _returnvalue 0.5 _returnvalue (`self.K2_GetActorLocation` _returnvalue) 10.0 "None")
        (goto _label :!via `Reverse`)))))

(fn `UserConstructionScript`)